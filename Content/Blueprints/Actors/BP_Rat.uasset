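; Player-controlled rat pawn that uses Enhanced Input for movement and a single action, adding the default mapping context on BeginPlay.
; Move input drives world-axis movement and snaps the mesh to face the input direction with a 90-degree offset.
; Action input only raises an IsActionActive flag for the ActionCooldown duration, ignoring repeat presses until it clears.
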(event `self.ReceiveBeginPlay`
  (bind _asplayer_controller (cast `PlayerController` (`self.GetController`)))
  (bind _returnvalue (pcsubsystem `EnhancedInputLocalPlayerSubsystem` _asplayer_controller))
  (`/Engine/EditorBlueprintResources/StandardMacros.IsValid` _returnvalue
    (:`Is Valid`
      (`EnhancedInputSubsystemInterface.AddMappingContext` _returnvalue "/Game/Inputs/IMC_Default.IMC_Default" 0 (struct)))))

(event `EnhancedInput|/Game/Inputs/IA_Move`
  (params (ActionValue :type "Vector2D Structure") (ElapsedSeconds :type "Float (double-precision)") (TriggeredSeconds :type "Float (double-precision)") (InputAction :type "InputAction Object Reference" :default "/Game/Inputs/IA_Move.IA_Move"))
  (:`Triggered`
    (`self.AddMovementInput` (`KismetMathLibrary.MakeVector` ActionValue_X ActionValue_Y))
    (`SceneComponent.K2_SetWorldRotation` (`self.Mesh`) (`KismetMathLibrary.ComposeRotators` (`KismetMathLibrary.MakeRotFromX` (`KismetMathLibrary.MakeVector` ActionValue_X ActionValue_Y)) (struct :`Yaw` -90.0)) false false)))

(event `EnhancedInput|/Game/Inputs/IA_Action`
  (params (ActionValue :type Boolean) (ElapsedSeconds :type "Float (double-precision)") (TriggeredSeconds :type "Float (double-precision)") (InputAction :type "InputAction Object Reference" :default "/Game/Inputs/IA_Action.IA_Action"))
  (:`Started`
    (if (and ActionValue (not (`self.IsActionActive`)))
      (set `self.IsActionActive` true)
      (`KismetSystemLibrary.Delay` (`self.ActionCooldown`))
      (set `self.IsActionActive` false))))

(fn `UserConstructionScript`)