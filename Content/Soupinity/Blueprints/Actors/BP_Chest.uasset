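; BP_Chest is a loot container that AI bots can steal from, showing text for whether it holds an item.
; Inventory add and take events are bound at construction, and visuals follow whether the inventory is empty.
; A non-empty chest registers with the Rat GameState shortly after BeginPlay.
; A bot entering the detection sphere triggers looting on its AI controller, empties the chest and reports theft; leaving clears the controller's chest reference.
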(event `self.ReceiveBeginPlay`
  (`KismetSystemLibrary.Delay` 0.2)
  (`self.UpdateVisual`)
  (if (not (`/Game/Soupinity/Blueprints/Actors/Components/BP_InventoryComponent.IsEmpty` (`self.BP_InventoryComponent`)))
    (`/Game/Soupinity/Blueprints/GameFramework/BP_GameState.RegisterItem` (`/Game/Soupinity/Blueprints/Misc/BP_Library.GetRatGameState`))))

(event `HandleItemMove`
  (params (ItemTag :type "GameplayTag Structure") (TotalWeight :type "Float (double-precision)"))
  (`self.UpdateVisual`))

(event `self.Sphere.OnComponentBeginOverlap`
  (params (OverlappedComponent :type "PrimitiveComponent Object Reference") (OtherActor :type "Actor Object Reference") (OtherComp :type "PrimitiveComponent Object Reference") (OtherBodyIndex :type Integer) (bFromSweep :type Boolean) (SweepResult :type "HitResult Structure (by ref)"))
  (bind _asbp_bot (cast `/Game/Soupinity/AI/Bot/BP_Bot` OtherActor))
  (bind _asaic_bot (cast `/Game/Soupinity/AI/Bot/AIC_Bot` (`AIBlueprintHelperLibrary.GetAIController` _asbp_bot)))
  (if (not (`/Game/Soupinity/Blueprints/Actors/Components/BP_InventoryComponent.IsEmpty` (`self.BP_InventoryComponent`)))
    (set `/Game/Soupinity/AI/Bot/AIC_Bot.Chest` self _asaic_bot)
    (`/Game/Soupinity/AI/Bot/AIC_Bot.HandleLooting` _asaic_bot)
    (`/Game/Soupinity/Blueprints/Actors/Components/BP_InventoryComponent.RemoveItems` (`self.BP_InventoryComponent`))
    (`/Game/Soupinity/Blueprints/GameFramework/BP_GameState.HandleItemTheft` (`/Game/Soupinity/Blueprints/Misc/BP_Library.GetRatGameState`))))

(event `self.Sphere.OnComponentEndOverlap`
  (params (OverlappedComponent :type "PrimitiveComponent Object Reference") (OtherActor :type "Actor Object Reference") (OtherComp :type "PrimitiveComponent Object Reference") (OtherBodyIndex :type Integer))
  (bind _asbp_bot (cast `/Game/Soupinity/AI/Bot/BP_Bot` OtherActor))
  (bind _asaic_bot (cast `/Game/Soupinity/AI/Bot/AIC_Bot` (`AIBlueprintHelperLibrary.GetAIController` _asbp_bot)))
  (set `/Game/Soupinity/AI/Bot/AIC_Bot.Chest` null _asaic_bot)
  (`/Game/Soupinity/AI/Bot/AIC_Bot.HandleLooting` _asaic_bot))

(fn `AddItemToContainer`
  (params (Instigator :type "Pawn Object Reference") (Item :type "/Game/Soupinity/Blueprints/Actors/Items/FItemInfo Structure"))
  (returns (Success :type Boolean)))

(fn `GetPossibleInteraction`
  (params (Instigator :type "Pawn Object Reference"))
  (returns (PossibleInteraction :type "/Game/Soupinity/Blueprints/Actors/Pawns/ENUM_Interaction Enum"))
  (return (select `bool` (`/Game/Soupinity/Blueprints/Actors/Components/BP_InventoryComponent.IsEmpty` (`self.BP_InventoryComponent`)) :`false` "NewEnumerator1" :`true` "NewEnumerator2" :!type "/Game/Soupinity/Blueprints/Actors/Pawns/ENUM_Interaction Enum")))

(fn `MoveItem`
  (params (Pawn :type "Pawn Object Reference")))

(fn `NewFunction`)

(fn `TakeItemFromContainer`
  (params (Instigator :type "Pawn Object Reference"))
  (returns (Item :type "/Game/Soupinity/Blueprints/Actors/Items/FItemInfo Structure")))

(fn `UpdateVisual`
  (bind _possibleinteraction (`self.GetPossibleInteraction` null))
  (switch `/Game/Soupinity/Blueprints/Actors/Pawns/ENUM_Interaction` _possibleinteraction
    (:`NewEnumerator1`
      (`SceneComponent.SetVisibility` (`self.GotItemText`) true false)
      (`SceneComponent.SetVisibility` (`self.EmptyText`) false false))
    (:`NewEnumerator2`
      (`SceneComponent.SetVisibility` (`self.GotItemText`) false false)
      (`SceneComponent.SetVisibility` (`self.EmptyText`) true false))))

(fn `UserConstructionScript`
  (bind _bp_inventorycomponent (`self.BP_InventoryComponent`))
  (`self.UpdateVisual`)
  (add `/Game/Soupinity/Blueprints/Actors/Components/BP_InventoryComponent.OnItemAdded` _bp_inventorycomponent (`|CreateDelegate` :!event `HandleItemMove`))
  (add `/Game/Soupinity/Blueprints/Actors/Components/BP_InventoryComponent.OnItemTaken` _bp_inventorycomponent (`|CreateDelegate` :!event `HandleItemMove`))
  (`SphereComponent.SetSphereRadius` (`self.Sphere`) (`self.AIDetectionRadius`) true))