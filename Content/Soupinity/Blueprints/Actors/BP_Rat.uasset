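; BP_Rat is the player-controlled rat, which moves with Enhanced Input and carries one item at a time between interactable actors.
; A cooldown-gated action sphere-traces for a BPI_Interaction actor to take or put an item, with a light showing the carried item's color.
; Each tick, stamina regenerates at rest or drains otherwise, scaled by HeavyCoef when carrying, and a curve table converts it into the movement speed coefficient.
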(event `self.ReceiveTick`
  (params (DeltaSeconds :type "Float (single-precision)"))
  (`self.UpdateStamina` DeltaSeconds))

(event `self.ReceiveBeginPlay`
  (bind _asplayer_controller (cast `PlayerController` (`self.GetController`)))
  (bind _returnvalue (pcsubsystem `EnhancedInputLocalPlayerSubsystem` _asplayer_controller))
  (`/Engine/EditorBlueprintResources/StandardMacros.IsValid` _returnvalue
    (:`Is Valid`
      (`EnhancedInputSubsystemInterface.AddMappingContext` _returnvalue "/Game/Soupinity/Inputs/IMC_Default.IMC_Default" 0 (struct)))))

(event `EnhancedInput|/Game/Soupinity/Inputs/IA_Move`
  (params (ActionValue :type "Vector2D Structure") (ElapsedSeconds :type "Float (double-precision)") (TriggeredSeconds :type "Float (double-precision)") (InputAction :type "InputAction Object Reference" :default "/Game/Soupinity/Inputs/IA_Move.IA_Move"))
  (bind _speedcoef (`self.SpeedCoef`))
  (:`Triggered`
    (`self.AddMovementInput` (`KismetMathLibrary.MakeVector` (* ActionValue_X _speedcoef) (* _speedcoef ActionValue_Y)))
    (`SceneComponent.K2_SetWorldRotation` (`self.Mesh`) (`KismetMathLibrary.ComposeRotators` (`KismetMathLibrary.MakeRotFromX` (`KismetMathLibrary.MakeVector` ActionValue_X ActionValue_Y)) (struct :`Yaw` -90.0)) false false)))

(event `EnhancedInput|/Game/Soupinity/Inputs/IA_Action`
  (params (ActionValue :type Boolean) (ElapsedSeconds :type "Float (double-precision)") (TriggeredSeconds :type "Float (double-precision)") (InputAction :type "InputAction Object Reference" :default "/Game/Soupinity/Inputs/IA_Action.IA_Action"))
  (:`Started`
    (if (and ActionValue (not (`self.IsActionActive`)))
      (set `self.IsActionActive` true)
      (`self.TryInteract`)
      (`KismetSystemLibrary.Delay` (`self.ActionCooldown`))
      (set `self.IsActionActive` false))))

(event `TryInteract`
  (bind _returnvalue (`self.K2_GetActorLocation`))
  (bind _item_name (break `/Game/Soupinity/Blueprints/Actors/Items/F_Item` (`self.Item`)))
  (bind _item_name_2 (break `/Game/Soupinity/Blueprints/Actors/Items/F_Item` (`self.Item`)))
  (bind _item_name_3 (break `/Game/Soupinity/Blueprints/Actors/Items/F_Item` (`self.Item`)))
  (bind _outhit (`KismetSystemLibrary.SphereTraceSingleForObjects` _returnvalue _returnvalue 100.0 (`|MakeArray` "ObjectTypeQuery2" :!type "EObjectTypeQuery Enum")))
  (if (`GameplayStatics.BreakHitResult` _outhit)
    (bind _asbpi_interaction (cast `/Game/Soupinity/Blueprints/Actors/BPI_Interaction` (`.HitActor` (`GameplayStatics.BreakHitResult` _outhit))))
    (bind _possibleinteraction (`/Game/Soupinity/Blueprints/Actors/BPI_Interaction.GetPossibleInteraction` _asbpi_interaction self))
    (switch `/Game/Soupinity/Blueprints/Actors/ENUM_Interaction` _possibleinteraction
      (:`NewEnumerator1`
        (if (== _item_name_2 "None")
          (bind _item (`/Game/Soupinity/Blueprints/Actors/BPI_Interaction.GetItem` _asbpi_interaction self))
          (bind _output_get (set `self.Item` _item))
          (`LightComponent.SetLightColor` (`self.ItemLight`) (`KismetMathLibrary.Conv_ColorToLinearColor` (`.Color_5_262A83EF467DE0418B98A4B45484B026` (break `/Game/Soupinity/Blueprints/Actors/Items/F_Item` _output_get))) true)
          (`SceneComponent.SetVisibility` (`self.ItemLight`) true false)
          (`KismetSystemLibrary.PrintString` (`KismetStringLibrary.Concat_StrStr` "This is " (`KismetStringLibrary.Conv_NameToString` (break `/Game/Soupinity/Blueprints/Actors/Items/F_Item` _output_get)) "!"))))
      (:`NewEnumerator2`
        (if (not (== _item_name "None"))
          (`SceneComponent.SetVisibility` (`self.ItemLight`) false false)
          (`KismetSystemLibrary.PrintString` (`KismetStringLibrary.Concat_StrStr` "You saved the " (`KismetStringLibrary.Conv_NameToString` _item_name_3) "!"))
          (`/Game/Soupinity/Blueprints/Actors/BPI_Interaction.AddItem` _asbpi_interaction self (`self.Item`))
          (set `self.Item` (make `/Game/Soupinity/Blueprints/Actors/Items/F_Item` "None" (make `Color` 0))))))))

(fn `AdjustMovementSpeed`
  (bind _outxy (`DataTableFunctionLibrary.EvaluateCurveTableRow` "/Game/Soupinity/Blueprints/Actors/CurveTable_Misc.CurveTable_Misc" "DelayedFastOut" (- 1.0 (/ (`self.Stamina`) 100.0)))
    (:`RowFound`
      (set `self.SpeedCoef` _outxy))))

(fn `UpdateStamina`
  (params (DeltaSeconds :type "Float (double-precision)"))
  (returns (UpdatedValue :type "Float (double-precision)"))
  (locals (TMP :type "Float (double-precision)" :default 0.0))
  (bind _item (`self.Item`))
  (`|ExecutionSequence`
    (:`then_0`
      (if (and (< (`KismetMathLibrary.VSize` (`self.GetVelocity`)) 1.0) (< (`KismetMathLibrary.VSize` (`KismetMathLibrary.Conv_Vector2DToVector` (`|GetInputActionValue`))) 0.1))
        (set `local.TMP` (`self.StaminaRegenSpeed`))
        (elif (!= (+ (break `Color` (`.Color_5_262A83EF467DE0418B98A4B45484B026` (break `/Game/Soupinity/Blueprints/Actors/Items/F_Item` _item))) (`.G` (break `Color` (`.Color_5_262A83EF467DE0418B98A4B45484B026` (break `/Game/Soupinity/Blueprints/Actors/Items/F_Item` _item)))) (`.R` (break `Color` (`.Color_5_262A83EF467DE0418B98A4B45484B026` (break `/Game/Soupinity/Blueprints/Actors/Items/F_Item` _item)))) (`.A` (break `Color` (`.Color_5_262A83EF467DE0418B98A4B45484B026` (break `/Game/Soupinity/Blueprints/Actors/Items/F_Item` _item))))) 0)
          (set `local.TMP` (* (`self.StaminaDrainSpeed`) (`self.HeavyCoef`)))
          (else
            (set `local.TMP` (`self.StaminaDrainSpeed`))))))
    (:`then_1`
      (bind _output_get (set `self.Stamina` (`KismetMathLibrary.FClamp` (+ (`self.Stamina`) (* DeltaSeconds (`local.TMP`))) 0.0 100.0)))
      (`self.AdjustMovementSpeed`)
      (return _output_get))))

(fn `UserConstructionScript`)