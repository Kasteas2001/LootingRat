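; Inventory component that stores item tags up to a capacity and totals their weight from per-tag item info.
; Adding and taking from the front recalculate weight and fire notifications with the tag and total.
; On BeginPlay it attempts to trim oversized lists set up in the level.
; Transfers move one item into an empty inventory, reporting theft to the Rat GameState when the receiving pawn is not player-controlled.
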(event `self.ReceiveBeginPlay`
  ;[1 1 1] Если кто вдруг добавит больше предметов, чем нужно на карте
  (`self.ResizeInnventory`)
  (`self.CalculateWeight`))

(fn `CalculateWeight`
  (returns (TotalWeight :type "Float (double-precision)"))
  (set `self.TotalWeight` 0.0)
  (for _array_element (`self.Items`)
    (bind (_iteminfo_name _iteminfo_color _iteminfo_weight) (break `/Game/Soupinity/Blueprints/Actors/Items/FItemInfo` (`/Game/Soupinity/Blueprints/Misc/BP_Library.Get Item Info for Tag` _array_element)))
    (set `self.TotalWeight` (+ (`self.TotalWeight`) _iteminfo_weight)))
  (return (`self.TotalWeight`)))

(fn `IsEmpty`
  (returns (Result :type Boolean))
  (return (`KismetArrayLibrary.Array_IsEmpty` (`self.Items`))))

(fn `MoveItemToAnotherComponent`
  (params (TargetInventoryComponent :type "/Game/Soupinity/Blueprints/Actors/Components/BP_InventoryComponent Object Reference"))
  (returns (Success :type Boolean))
  (if (and (not (`self.IsEmpty`)) (`self.IsEmpty` TargetInventoryComponent))
    (`|ExecutionSequence`
      (:`then_0`
        (bind _aspawn (cast `Pawn` (`self.GetOwner` (`local.TargetInventoryComponent`))))
        (if (not (`Pawn.IsPlayerControlled` _aspawn))
          (`/Game/Soupinity/Blueprints/GameFramework/BP_GameState.HandleItemTheft` (`/Game/Soupinity/Blueprints/Misc/BP_Library.GetRatGameState`))))
      (:`then_1`
        (bind _item (`self.TakeItem`))
        (`self.TryAddItem` (`local.TargetInventoryComponent`) _item)
        (return true)))
    (else
      (return false))))

(fn `RemoveItems`
  (`KismetArrayLibrary.Array_Clear` (`self.Items`)))

(fn `ResizeInnventory`
  (bind _returnvalue (`KismetArrayLibrary.Array_Length` (`self.Items`)))
  (if (> _returnvalue (`self.InvetorySize`))
    (for _index (range 1 _returnvalue)
      (`KismetArrayLibrary.Array_Remove` (`self.Items`) _index))))

(fn `TakeItem`
  (returns (Item :type "GameplayTag Structure"))
  (locals (TMPItem :type "GameplayTag Structure"))
  (bind _items (`self.Items`))
  (bind _tmpitem (`local.TMPItem`))
  (if (`KismetArrayLibrary.Array_IsValidIndex` _items)
    (set `local.TMPItem` (`|GetArrayItem` _items))
    (`KismetArrayLibrary.Array_Remove` (`self.Items`))
    (bind _totalweight (`self.CalculateWeight`))
    (`self.OnItemTaken` _tmpitem _totalweight)
    (return _tmpitem)))

(fn `TryAddItem`
  (params (Item :type "GameplayTag Structure"))
  (returns (Success :type Boolean))
  (if (< (`KismetArrayLibrary.Array_Length` (`self.Items`)) (`self.InvetorySize`))
    (`KismetArrayLibrary.Array_Add` (`self.Items`) (`local.Item`))
    (bind _totalweight (`self.CalculateWeight`))
    (`self.OnItemAdded` (`local.Item`) _totalweight)
    (return true)
    (else
      (return false))))