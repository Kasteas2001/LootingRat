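; BP_HeroSpawnManager is an actor that triggers timed spawns at BP_Gate actors, scheduled by a data table.
; On BeginPlay it copies the table rows into spawn entries and starts a looping one-second timer.
; Each tick advances and prints a time counter, removes due entries, and calls Spawn on gates with matching tags.
; The gate list comes from GetAllGates, which nothing in this Blueprint calls.
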(event `GetAllGates`
  (bind _outactors (`GameplayStatics.GetAllActorsOfClass` "/Game/Soupinity/Blueprints/Actors/BP_Gate.BP_Gate_C"))
  (set `self.Gates` _outactors))

(event `InitSpawnEntries`
  (bind _datatable (`self.DataTable`))
  (bind _outrownames (`DataTableFunctionLibrary.GetDataTableRowNames` _datatable))
  (for _array_element _outrownames
    (bind _returnvalue (`|GetDataTableRow` _datatable _array_element)
      (:`then`
        (bind (_gatetag _timebeforespawn) (break `/Game/Soupinity/Blueprints/Misc/FSpawnEntry` _returnvalue))
        (`KismetArrayLibrary.Array_Add` (`self.SpawnEntries`) (make `/Game/Soupinity/Blueprints/Misc/FSpawnEntry` _gatetag _timebeforespawn))))))

(event `self.ReceiveBeginPlay`
  (`self.InitSpawnEntries`)
  (bind _returnvalue (`KismetSystemLibrary.K2_SetTimerDelegate` (delegate `TryToSpawn`) 1.0 true))
  (set `self.SpawnCheckTimer` _returnvalue)
  (set `self.Time` 0.0))

(event `TryToSpawn`
  (bind _result (`/Engine/EditorBlueprintResources/StandardMacros.IncrementFloat` (`self.Time`))
    (:`  `
      (`KismetSystemLibrary.PrintString` (`KismetStringLibrary.Conv_DoubleToString` _result))
      (bind _poppedentries (`self.PopSuitableEntries`))
      (for _array_element _poppedentries
        (for _array_element_2 (`self.Gates`)
          (if (== (break `/Game/Soupinity/Blueprints/Misc/FSpawnEntry` _array_element) (`/Game/Soupinity/Blueprints/Actors/BP_Gate.Tag` _array_element_2))
            (`/Game/Soupinity/Blueprints/Actors/BP_Gate.Spawn` _array_element_2)))))))

(fn `PopSuitableEntries`
  (returns (PoppedEntries :type "Array of /Game/Soupinity/Blueprints/Misc/FSpawnEntry Structure"))
  (locals (TMP :type "Array of /Game/Soupinity/Blueprints/Misc/FSpawnEntry Structure"))
  (for _array_element (`self.SpawnEntries`)
    (if (<= (`.TimeBeforeSpawn_6_6282F1CB4FD12E94B8156FB8711DC5CA` (break `/Game/Soupinity/Blueprints/Misc/FSpawnEntry` _array_element)) (`self.Time`))
      (`KismetArrayLibrary.Array_Add` (`local.TMP`) _array_element)))
  (for _array_element_2 (`local.TMP`)
    (`KismetArrayLibrary.Array_RemoveItem` (`self.SpawnEntries`) _array_element_2))
  (return (`local.TMP`)))

(fn `UserConstructionScript`)