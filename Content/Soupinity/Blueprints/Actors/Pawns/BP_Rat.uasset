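; BP_Rat is the player-controlled rat pawn, which moves with Enhanced Input, carries items and plays a death animation when its health component signals death.
; Each tick updates stamina from movement and carried load, then maps it through a curve table to scale movement input.
; The action input, gated by a cooldown, finds the nearest BPI_Interaction actor by sphere trace to take, put or use.
; Inventory events drive an item light and debug messages.
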(event `self.ReceiveTick`
  (params (DeltaSeconds :type "Float (single-precision)"))
  (`self.UpdateStamina` DeltaSeconds))

(event `self.ReceiveBeginPlay`
  (`|ExecutionSequence`
    (:`then_0`
      (bind _asplayer_controller (cast `PlayerController` (`self.GetController`)))
      (bind _returnvalue (pcsubsystem `EnhancedInputLocalPlayerSubsystem` _asplayer_controller))
      (`/Engine/EditorBlueprintResources/StandardMacros.IsValid` _returnvalue
        (:`Is Valid`
          (`EnhancedInputSubsystemInterface.AddMappingContext` _returnvalue "/Game/Soupinity/Inputs/IMC_Default.IMC_Default" 0 (struct)))))
    (:`then_1`
      (add `/Game/Soupinity/Blueprints/Actors/Components/BP_HealthComponent.OnDeath` (`self.BP_HealthComponent`) (`|CreateDelegate` :!event `EventOnDeath`)))))

(event `EventOnDeath`
  (`CharacterMovementComponent.DisableMovement` (`self.CharacterMovement`))
  (`SkeletalMeshComponent.PlayAnimation` (`self.Mesh`) "/Game/Soupinity/Animations/Rat/Anim_Death.Anim_Death" false))

(event `EnhancedInput|/Game/Soupinity/Inputs/IA_Move`
  (params (ActionValue :type "Vector2D Structure") (ElapsedSeconds :type "Float (double-precision)") (TriggeredSeconds :type "Float (double-precision)") (InputAction :type "InputAction Object Reference" :default "/Game/Soupinity/Inputs/IA_Move.IA_Move"))
  (bind _speedcoef (`self.SpeedCoef`))
  (:`Triggered`
    (`self.AddMovementInput` (`KismetMathLibrary.MakeVector` (* ActionValue_X _speedcoef) (* _speedcoef ActionValue_Y)))
    (`SceneComponent.K2_SetWorldRotation` (`self.Mesh`) (`KismetMathLibrary.ComposeRotators` (`KismetMathLibrary.MakeRotFromX` (`KismetMathLibrary.MakeVector` ActionValue_X ActionValue_Y)) (struct :`Yaw` -90.0)) false false)))

(event `ShowItemAdded`
  (params (ItemTag :type "GameplayTag Structure") (TotalWeight :type "Float (double-precision)"))
  (bind (_iteminfo_name _iteminfo_color) (break `/Game/Soupinity/Blueprints/Actors/Items/FItemInfo` (`/Game/Soupinity/Blueprints/Misc/BP_Library.Get Item Info for Tag` ItemTag)))
  (`LightComponent.SetLightColor` (`self.ItemLight`) _iteminfo_color true)
  (`SceneComponent.SetVisibility` (`self.ItemLight`) true false)
  (`KismetSystemLibrary.PrintString` (`KismetStringLibrary.Concat_StrStr` "This is " (`KismetStringLibrary.Conv_NameToString` _iteminfo_name) "!")))

(event `EnhancedInput|/Game/Soupinity/Inputs/IA_Action`
  (params (ActionValue :type Boolean) (ElapsedSeconds :type "Float (double-precision)") (TriggeredSeconds :type "Float (double-precision)") (InputAction :type "InputAction Object Reference" :default "/Game/Soupinity/Inputs/IA_Action.IA_Action"))
  (:`Started`
    (if (and ActionValue (not (`self.IsActionActive`)))
      (set `self.IsActionActive` true)
      (`self.TryInteract`)
      (`KismetSystemLibrary.Delay` (`self.ActionCooldown`))
      (set `self.IsActionActive` false))))

(event `ShowItemTaken`
  (params (ItemTag :type "GameplayTag Structure") (TotalWeight :type "Float (double-precision)"))
  (bind _iteminfo_name (break `/Game/Soupinity/Blueprints/Actors/Items/FItemInfo` (`/Game/Soupinity/Blueprints/Misc/BP_Library.Get Item Info for Tag` ItemTag)))
  (`LightComponent.SetLightColor` (`self.ItemLight`) (struct :`R` 1.0 :`G` 1.0 :`B` 1.0 :`A` 1.0) true)
  (`SceneComponent.SetVisibility` (`self.ItemLight`) true false)
  (`KismetSystemLibrary.PrintString` (`KismetStringLibrary.Concat_StrStr` "You saved the " (`KismetStringLibrary.Conv_NameToString` _iteminfo_name) "!")))

(event `TryInteract`
  (bind _nearestactor (`self.GetNearestActor`))
  (bind _bp_inventorycomponent (`self.BP_InventoryComponent`))
  (bind _returnvalue (`self.GetComponentByClass` _nearestactor "/Game/Soupinity/Blueprints/Actors/Components/BP_InventoryComponent.BP_InventoryComponent_C"))
  (bind _asbpi_interaction (cast `/Game/Soupinity/Blueprints/Interfaces/BPI_Interaction` _nearestactor))
  (bind _possibleinteraction (`/Game/Soupinity/Blueprints/Interfaces/BPI_Interaction.GetPossibleInteraction` _asbpi_interaction self))
  (switch `/Game/Soupinity/Blueprints/Actors/Pawns/ENUM_Interaction` _possibleinteraction
    (:`NewEnumerator1`
      (`/Game/Soupinity/Blueprints/Actors/Components/BP_InventoryComponent.MoveItemToAnotherComponent` _returnvalue _bp_inventorycomponent))
    (:`NewEnumerator2`
      (`/Game/Soupinity/Blueprints/Actors/Components/BP_InventoryComponent.MoveItemToAnotherComponent` _bp_inventorycomponent _returnvalue))
    (:`NewEnumerator3`
      (`/Game/Soupinity/Blueprints/Interfaces/BPI_Interaction.Interact` _asbpi_interaction self))))

(fn `AdjustMovementSpeed`
  (bind _outxy (`DataTableFunctionLibrary.EvaluateCurveTableRow` "/Game/Soupinity/Blueprints/Misc/CurveTable_Misc.CurveTable_Misc" "DelayedFastOut" (- 1.0 (/ (`self.Stamina`) 100.0)))
    (:`RowFound`
      (set `self.SpeedCoef` _outxy))))

(fn `GetNearestActor`
  (returns (NearestActor :type "Actor Object Reference"))
  (locals (ClosestDistance :type "Float (double-precision)" :default 999999999.0) (TmpClosestActor :type "Actor Object Reference"))
  (bind _returnvalue (`self.K2_GetActorLocation`))
  (bind _outhits (`KismetSystemLibrary.SphereTraceMultiForObjects` _returnvalue _returnvalue 100.0 (`|MakeArray` "ObjectTypeQuery2" :!type "EObjectTypeQuery Enum")))
  (for _array_element _outhits
    (bind _returnvalue_2 (`self.GetDistanceTo` (`.HitActor` (`GameplayStatics.BreakHitResult` _array_element)) self))
    (if (and (< _returnvalue_2 (`local.ClosestDistance`)) (`KismetSystemLibrary.DoesImplementInterface` (`.HitActor` (`GameplayStatics.BreakHitResult` _array_element)) "/Game/Soupinity/Blueprints/Interfaces/BPI_Interaction.BPI_Interaction_C"))
      (set `local.ClosestDistance` _returnvalue_2)
      (set `local.TmpClosestActor` (`.HitActor` (`GameplayStatics.BreakHitResult` _array_element)))))
  (return (`local.TmpClosestActor`)))

(fn `UpdateStamina`
  (params (DeltaSeconds :type "Float (double-precision)"))
  (returns (UpdatedValue :type "Float (double-precision)"))
  (locals (TMP :type "Float (double-precision)" :default 0.0))
  (`|ExecutionSequence`
    (:`then_0`
      (if (and (< (`KismetMathLibrary.VSize` (`self.GetVelocity`)) 1.0) (< (`KismetMathLibrary.VSize` (`KismetMathLibrary.Conv_Vector2DToVector` (`|GetInputActionValue`))) 0.1))
        (set `local.TMP` (`self.StaminaRegenSpeed`))
        (elif (not (`/Game/Soupinity/Blueprints/Actors/Components/BP_InventoryComponent.IsEmpty` (`self.BP_InventoryComponent`)))
          (set `local.TMP` (* (`self.StaminaDrainSpeed`) (`self.HeavyCoef`)))
          (else
            (set `local.TMP` (`self.StaminaDrainSpeed`))))))
    (:`then_1`
      (bind _output_get (set `self.Stamina` (`KismetMathLibrary.FClamp` (+ (`self.Stamina`) (* DeltaSeconds (`local.TMP`))) 0.0 100.0)))
      (`self.AdjustMovementSpeed`)
      (return _output_get))))

(fn `UserConstructionScript`
  (bind _bp_inventorycomponent (`self.BP_InventoryComponent`))
  (add `/Game/Soupinity/Blueprints/Actors/Components/BP_InventoryComponent.OnItemAdded` _bp_inventorycomponent (`|CreateDelegate` :!event `ShowItemAdded`))
  (add `/Game/Soupinity/Blueprints/Actors/Components/BP_InventoryComponent.OnItemTaken` _bp_inventorycomponent (`|CreateDelegate` :!event `ShowItemTaken`)))