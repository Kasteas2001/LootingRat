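; BP_Gate is a spawn point actor that creates BP_Bot instances through its Spawn event.
; Each spawn plays a SimpleExplosion effect at the gate and hands the bot a random entry from AISplines.
; With no splines assigned, it only prints a debug message identifying the gate by its gameplay tag.
; Nothing inside this Blueprint triggers Spawn, as BeginPlay, overlap and Tick are unused.
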(event `Spawn`
  (bind (_returnvalue_location _returnvalue_rotation) (`KismetMathLibrary.BreakTransform` (`self.GetTransform`)))
  (if (`KismetArrayLibrary.Array_IsEmpty` (`self.AISplines`))
    (`KismetSystemLibrary.PrintString` (`KismetStringLibrary.Concat_StrStr` "No Splines at " (`BlueprintGameplayTagLibrary.GetDebugStringFromGameplayTag` (`self.Tag`))))
    (else
      (`KismetSystemLibrary.PrintString` (`KismetStringLibrary.Concat_StrStr` "Spawn at " (`BlueprintGameplayTagLibrary.GetDebugStringFromGameplayTag` (`self.Tag`))))
      (`NiagaraFunctionLibrary.SpawnSystemAtLocation` "/Niagara/DefaultAssets/Templates/Systems/SimpleExplosion.SimpleExplosion" (`self.K2_GetActorLocation`))
      (`|SpawnActorFromClass` "/Game/Soupinity/AI/Bot/BP_Bot.BP_Bot_C" (`KismetMathLibrary.MakeTransform` _returnvalue_location _returnvalue_rotation) "Undefined" "OverrideRootScale" null (`KismetArrayLibrary.Array_Random` (`self.AISplines`)) null))))

(fn `UserConstructionScript`)