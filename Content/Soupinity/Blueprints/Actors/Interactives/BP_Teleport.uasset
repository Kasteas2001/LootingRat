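; BP_Teleport is an interactive actor that moves whoever interacts with it to the location of a linked OtherTeleport.
; Interact fades the camera out, holds through a delay scaled from FadeDelay, then starts the fade back in and immediately teleports the instigator without sweeping.
; GetPossibleInteraction reports a fixed interaction type, and GetItem is an empty stub.
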(event `/Game/Soupinity/Blueprints/Interfaces/BPI_Interaction.Interact`
  (params (Instigator :type "Pawn Object Reference"))
  (`PlayerCameraManager.StartCameraFade` :`self` (`GameplayStatics.GetPlayerCameraManager` 0) :`ToAlpha` 1.0 :`Duration` (`self.FadeDelay`) :`bHoldWhenFinished` true)
  (`KismetSystemLibrary.Delay` (* (`self.FadeDelay`) 1.5))
  (`PlayerCameraManager.StartCameraFade` :`self` (`GameplayStatics.GetPlayerCameraManager` 0) :`FromAlpha` 1.0 :`ToAlpha` 0.0 :`Duration` (`self.FadeDelay`))
  (`self.K2_SetActorLocation` Instigator (`self.K2_GetActorLocation` (`self.OtherTeleport`)) false true))

(fn `GetItem`
  (params (Instigator :type "Pawn Object Reference"))
  (returns (Item :type "/Game/Soupinity/Blueprints/Actors/Items/F_Item Structure"))
  (return))

(fn `GetPossibleInteraction`
  (params (Instigator :type "Pawn Object Reference"))
  (returns (PossibleInteraction :type "/Game/Soupinity/Blueprints/Actors/Pawns/ENUM_Interaction Enum"))
  (return "NewEnumerator3"))

(fn `UserConstructionScript`)