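; Spline path actor that draws arrows along its route, likely for AI paths going by its name, and is hidden until toggled.
; The construction script tiles spline meshes at fixed section lengths, clamping tangents to that length, then nudges them upward and hides them.
; All sections share one dynamic arrow material driven by speed, emissive and color variables.
; The TurnVisualon event shows or hides every section.
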(event `self.TurnVisualOn`
  (params (NewParam :type Boolean))
  (`self.SetSplineVisibility` NewParam))

(fn `InitMaterial`
  (bind _returnvalue (`KismetMaterialLibrary.CreateDynamicMaterialInstance` "/Game/Soupinity/Materials/Instances/MI_SplineArrows.MI_SplineArrows"))
  (bind _output_get (set `self.DynamicMaterial` _returnvalue))
  (`MaterialInstanceDynamic.SetScalarParameterValue` _output_get "Speed" (`self.Speed`))
  (`MaterialInstanceDynamic.SetScalarParameterValue` _output_get "Emissive" (`self.Emissive`))
  (`MaterialInstanceDynamic.SetVectorParameterValue` _output_get "Color" (`self.Color`)))

(fn `PositionAndTangentAtSplineLocation`
  (params (Index :type Integer))
  (returns (Position :type "Vector Structure") (Tangent :type "Vector Structure"))
  (bind _splinepath (`self.SplinePath`))
  (bind _returnvalue (* Index (`self.SectionLength`)))
  (return (`SplineComponent.GetLocationAtDistanceAlongSpline` _splinepath _returnvalue "Local") (`KismetMathLibrary.ClampVectorSize` (`SplineComponent.GetTangentAtDistanceAlongSpline` _splinepath _returnvalue "Local") 0.0 (`self.SectionLength`))))

(fn `SetSplineVisibility`
  (params (bNewVisibility :type Boolean))
  (for _array_element (`self.K2_GetComponentsByClass` "/Script/Engine.SplineMeshComponent")
    (`SceneComponent.SetVisibility` _array_element bNewVisibility false)))

(fn `UserConstructionScript`
  (locals (LoopIndex :type Integer))
  (`self.InitMaterial`)
  (for _index (range (+ (`KismetMathLibrary.FTrunc` (/ (`SplineComponent.GetSplineLength` (`self.SplinePath`)) (`self.SectionLength`))) 1))
    (set `local.LoopIndex` _index)
    (bind _returnvalue (`AddComponent|NODE_AddSplineMeshComponent-0`))
    (`PrimitiveComponent.SetMaterial` _returnvalue 0 (`self.DynamicMaterial`))
    (`StaticMeshComponent.SetStaticMesh` _returnvalue (`self.SplineMesh`))
    (`SplineMeshComponent.SetForwardAxis` _returnvalue "X" true)
    (bind (_position _tangent) (`self.PositionAndTangentAtSplineLocation` (`local.LoopIndex`)))
    (bind (_position_2 _tangent_2) (`self.PositionAndTangentAtSplineLocation` (+ (`local.LoopIndex`) 1)))
    (`SplineMeshComponent.SetStartAndEnd` _returnvalue _position _tangent _position_2 _tangent_2 true))
  (for _array_element (`self.K2_GetComponentsByClass` "/Script/Engine.SplineMeshComponent")
    (`SceneComponent.K2_AddWorldOffset` _array_element (0.0 0.0 0.1) false false)
    (`SceneComponent.SetVisibility` _array_element false false)))