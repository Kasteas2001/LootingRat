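; Melee enemy bot that repeatedly attacks while something is inside its MeleeAttackBox.
; Overlap begin plays the attack montage at once and starts a looping timer matched to montage length; any overlap end clears it.
; The montage's Deal Damage notify fires the OnPerformMeleeAttack dispatcher, bound on BeginPlay to apply the Weapon's base damage to every Pawn overlapping the box.
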(event `self.ReceiveBeginPlay`
  (add `self.OnPerformMeleeAttack` (delegate `OnPerformMeleeAttack_Event`)))

(event `OnPerformMeleeAttack_Event`
  (for _array_element (`PrimitiveComponent.GetOverlappingActors` (`self.MeleeAttackBox`) "/Script/Engine.Pawn")
    (bind _weapon (`self.Weapon`)
      (:`then`
        (`GameplayStatics.ApplyDamage` _array_element (`/Game/Soupinity/Blueprints/Weapons/BP_Weapon.BaseDamage` _weapon) (`self.GetController`) _weapon))
      (:`else`))))

(event `self.MeleeAttackBox.OnComponentBeginOverlap`
  (params (OverlappedComponent :type "PrimitiveComponent Object Reference") (OtherActor :type "Actor Object Reference") (OtherComp :type "PrimitiveComponent Object Reference") (OtherBodyIndex :type Integer) (bFromSweep :type Boolean) (SweepResult :type "HitResult Structure (by ref)"))
  (bind _meleeattackmontage (`self.MeleeAttackMontage`)
    (:`then`
      (bind _returnvalue (`KismetSystemLibrary.K2_SetTimerDelegate` (delegate `PerformMeleeAttack`) (`AnimationAsset.GetPlayLength` _meleeattackmontage) true))
      (set `self.MeleeAttackTimer` _returnvalue)
      (`self.PerformMeleeAttack`))
    (:`else`)))

(event `PerformMeleeAttack`
  (bind _notifyname (`|PlayMontage` (`self.Mesh`) (`self.MeleeAttackMontage`))
    (:`OnNotifyBegin`
      (switch `name` _notifyname
        (:`DealDamage`
          (`self.OnPerformMeleeAttack`))))))

(event `self.MeleeAttackBox.OnComponentEndOverlap`
  (params (OverlappedComponent :type "PrimitiveComponent Object Reference") (OtherActor :type "Actor Object Reference") (OtherComp :type "PrimitiveComponent Object Reference") (OtherBodyIndex :type Integer))
  (`KismetSystemLibrary.K2_ClearAndInvalidateTimerHandle` (`self.MeleeAttackTimer`)))

(fn `UserConstructionScript`
  (`parent.UserConstructionScript`))