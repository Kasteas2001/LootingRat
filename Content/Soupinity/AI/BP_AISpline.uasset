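; BP_AISpline is an actor that counts the pawns registered to it and signals when its visual turns on or off.
; RegistrPawn increments the count, binds to the pawn's OnDestroyed event and calls TurnVisualOn(true) while the count is positive.
; Each destroyed pawn decrements the count, switching the visual off at zero.
; TurnVisualOn is empty here, and no spline logic appears in the graphs.
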(event `RegistrPawn`
  (params (Pawn :type "Pawn Object Reference (by ref)"))
  (add `self.OnDestroyed` Pawn (delegate `CustomEvent`))
  (bind _result (`/Engine/EditorBlueprintResources/StandardMacros.IncrementInt` (`self.Pawns`))
    (:`  `
      (if (> _result 0)
        (`self.TurnVisualOn` true)))))

(event `CustomEvent` :!signature `self.OnDestroyed`
  (params (DestroyedActor :type "Actor Object Reference"))
  (bind _result (`/Engine/EditorBlueprintResources/StandardMacros.DecrementInt` (`self.Pawns`))
    (:`  `
      (if (<= _result 0)
        (`self.TurnVisualOn` false)))))

(event `TurnVisualOn`
  (params (NewParam :type Boolean)))

(fn `UserConstructionScript`)